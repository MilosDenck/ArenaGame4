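; BP_Enemy_Counter tracks how many living BP_Enemy_Master actors remain in the level.
; Every Tick it fetches all such actors, removes those flagged IsDead from that array during the loop, and increments KilledEnemies for each.
; When the remaining count differs from EnemyCount, it prints the new number and stores it.
; KilledEnemies accumulates every frame a dead actor still exists, so it is not a unique kill total.
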(event `self.ReceiveTick`
  (params (DeltaSeconds :type "Float (single-precision)"))
  (bind _outactors (`GameplayStatics.GetAllActorsOfClass` "/Game/Blueprints/AI/BP_Enemy_Master.BP_Enemy_Master_C"))
  (for _array_element _outactors
    (if (`/Game/Blueprints/AI/BP_Enemy_Master.isDead?` _array_element)
      (`KismetArrayLibrary.Array_RemoveItem` _outactors _array_element)
      (set `self.killedEnemies` (+ (`self.killedEnemies`) 1))))
  (bind _returnvalue (`KismetArrayLibrary.Array_Length` _outactors))
  (if (!= _returnvalue (`self.EnemyCount`))
    (`KismetSystemLibrary.PrintText` (`KismetTextLibrary.Conv_IntToText` _returnvalue))
    (set `self.EnemyCount` _returnvalue)))

(fn `UserConstructionScript`)