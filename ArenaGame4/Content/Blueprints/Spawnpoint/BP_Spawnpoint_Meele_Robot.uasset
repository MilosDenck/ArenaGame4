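; Spawn point Blueprint for melee robot enemies, exposing a Spawn Enemies function.
; The function spawns one BP_Melee AI pawn at the root component's world location, leaving its EnemyCount and Delay inputs unused.
; It casts the result to BP_Enemy_Melee_AI_A and returns it, printing "Cast Failed" if that fails.
; The event graph holds only disabled placeholder events, so nothing here triggers spawning by itself.
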(fn `Spawn Enemies`
  (params (EnemyCount :type Integer) (Delay :type "Float (double-precision)"))
  (returns (Enemy :type "/Game/Blueprints/AI/BP_Enemy_Master Object Reference"))
  (bind _returnvalue (`AIBlueprintHelperLibrary.SpawnAIFromClass` "/Game/Blueprints/AI/BP_Melee_C.BP_Melee_C_C" null (`SceneComponent.K2_GetComponentLocation` (`self.DefaultSceneRoot`)) (struct) false null))
  (bind _asbp_enemy_melee_ai_a (cast `/Game/Blueprints/AI/BP_Enemy_Melee_AI_A` _returnvalue)
    (:`then`
      _)
    (:`CastFailed`
      (`KismetSystemLibrary.PrintText` "Cast Failed")))
  (return _asbp_enemy_melee_ai_a))

(fn `UserConstructionScript`
  (`parent.UserConstructionScript`))